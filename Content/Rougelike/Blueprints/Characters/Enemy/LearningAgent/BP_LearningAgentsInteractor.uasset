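; Learning Agents interactor that defines what a BP_Scorpion enemy agent observes and which actions it can take.
; Observes the Hero as a struct of location relative to the scorpion, health, mana and stamina, wrapped in a set observation.
; An exclusive union action chooses between Attack and Move.
; Attack always triggers a melee attack, ignoring its discrete index, while Move feeds a direction and speed into PerformMove.
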(fn `GatherAgentObservation`
  (params (InObservationObject :type "LearningAgentsObservationObject Object Reference") (AgentId :type Integer))
  (returns (OutObservationObjectElement :type "LearningAgentsObservationObjectElement Structure"))
  (locals (AI_Enemy :type "EnemyCharacter Object Reference"))
  (bind _returnvalue (`BaseCharacter.GetAbilitySystemComponent` (`self.Hero`)))
  (set `local.AI_Enemy` (`self.GetAgent` AgentId "/Game/Rougelike/Blueprints/Characters/Enemy/BP_Scorpion.BP_Scorpion_C"))
  (return (`LearningAgentsObservations.MakeSetObservation` (`local.InObservationObject`) (`|MakeSet` (`LearningAgentsObservations.MakeStructObservation` (`local.InObservationObject`) (`|MakeMap` "Location" (`LearningAgentsObservations.MakeLocationObservation` (`local.InObservationObject`) (`Actor.K2_GetActorLocation` (`self.Hero`)) (`Actor.GetTransform` (`local.AI_Enemy`)) 1000.0 "LocationObservation" false null) "Health" (`LearningAgentsObservations.MakeFloatObservation` (`local.InObservationObject`) (`.ReturnValue` (`AbilitySystemComponent.GetGameplayAttributeValue` _returnvalue (struct :`AttributeName` "Health" :`Attribute` "/Script/CapstoneProject.CharacterBaseAttributeSet:Health" :`AttributeOwner` "/Script/CoreUObject.Class'/Script/CapstoneProject.CharacterBaseAttributeSet'"))) 1.0 "FloatObservation" false null) "Mana" (`LearningAgentsObservations.MakeFloatObservation` (`local.InObservationObject`) (`.ReturnValue` (`AbilitySystemComponent.GetGameplayAttributeValue` _returnvalue (struct :`AttributeName` "Mana" :`Attribute` "/Script/CapstoneProject.CharacterBaseAttributeSet:Mana" :`AttributeOwner` "/Script/CoreUObject.Class'/Script/CapstoneProject.CharacterBaseAttributeSet'"))) 1.0 "FloatObservation" false null) "Stamina" (`LearningAgentsObservations.MakeFloatObservation` (`local.InObservationObject`) (`.ReturnValue` (`AbilitySystemComponent.GetGameplayAttributeValue` _returnvalue (struct :`AttributeName` "Stamina" :`Attribute` "/Script/CapstoneProject.CharacterBaseAttributeSet:Stamina" :`AttributeOwner` "/Script/CoreUObject.Class'/Script/CapstoneProject.CharacterBaseAttributeSet'"))) 1.0 "FloatObservation" false null) :!type "Name"))))))

(fn `PerformAgentAction`
  (params (InActionObject :type "LearningAgentsActionObject Object Reference") (InActionObjectElement :type "LearningAgentsActionObjectElement Structure (by ref)") (AgentId :type Integer))
  (locals (Scale :type "Float (single-precision)" :default 0.0) (Direction :type "Vector Structure" :default (0.0 0.0 0.0)))
  (set `self.Scorpion` (`self.GetAgent` AgentId "/Game/Rougelike/Blueprints/Characters/Enemy/BP_Scorpion.BP_Scorpion_C"))
  (bind (_outelementname _outelement) (`LearningAgentsActions.GetExclusiveUnionAction` (`local.InActionObject`) (`local.InActionObjectElement`)))
  (switch `name` _outelementname
    (:`Attack`
      (`LearningAgentsActions.GetExclusiveDiscreteAction` (`local.InActionObject`) _outelement "DiscreteExclusiveAction" false null)
      (`BaseCharacter.DoMeleeAttack` (`self.Scorpion`)))
    (:`Move`
      (bind _outelements (`LearningAgentsActions.GetStructAction` (`local.InActionObject`) _outelement))
      (`|ExecutionSequence`
        (:`then_0`
          (bind _outdirection (`LearningAgentsActions.GetDirectionAction` (`local.InActionObject`) (`BlueprintMapLibrary.Map_Find` _outelements "Direction") (`Actor.GetTransform` (`self.Scorpion`)) "DirectionAction" false null))
          (set `local.Direction` _outdirection))
        (:`then_1`
          (bind _outvalue (`LearningAgentsActions.GetFloatAction` (`local.InActionObject`) (`BlueprintMapLibrary.Map_Find` _outelements "Speed") 1.0 "FloatAction" false null))
          (set `local.Scale` _outvalue))
        (:`then_2`
          (`/Game/Rougelike/Blueprints/Characters/Enemy/BP_Scorpion.PerformMove` (`self.Scorpion`) (`local.Direction`) (`local.Scale`)))))))

(fn `SpecifyAgentAction`
  (params (InActionSchema :type "LearningAgentsActionSchema Object Reference"))
  (returns (OutActionSchemaElement :type "LearningAgentsActionSchemaElement Structure"))
  (return (`LearningAgentsActions.SpecifyExclusiveUnionAction` (`local.InActionSchema`) (`|MakeMap` "Attack" (`LearningAgentsActions.SpecifyExclusiveDiscreteAction` (`local.InActionSchema`) 4) "Move" (`LearningAgentsActions.SpecifyStructAction` (`local.InActionSchema`) (`|MakeMap` "Direction" (`LearningAgentsActions.SpecifyDirectionAction` (`local.InActionSchema`)) "Speed" (`LearningAgentsActions.SpecifyFloatAction` (`local.InActionSchema`)) :!type "Name")) :!type "Name"))))

(fn `SpecifyAgentObservation`
  (params (InObservationSchema :type "LearningAgentsObservationSchema Object Reference"))
  (returns (OutObservationSchemaElement :type "LearningAgentsObservationSchemaElement Structure"))
  (return (`LearningAgentsObservations.SpecifySetObservation` InObservationSchema (`LearningAgentsObservations.SpecifyStructObservation` InObservationSchema (`|MakeMap` "Location" (`LearningAgentsObservations.SpecifyLocationObservation` (`local.InObservationSchema`)) "Health" (`LearningAgentsObservations.SpecifyFloatObservation` (`local.InObservationSchema`)) "Mana" (`LearningAgentsObservations.SpecifyFloatObservation` (`local.InObservationSchema`)) "Stamina" (`LearningAgentsObservations.SpecifyFloatObservation` (`local.InObservationSchema`)) :!type "Name")) 10)))