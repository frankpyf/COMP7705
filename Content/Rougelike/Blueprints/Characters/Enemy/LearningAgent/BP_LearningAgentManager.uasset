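; Learning Agents manager actor that trains or runs the neural-network policy for Scorpion enemies.
; BeginPlay makes scorpions tick after it, then builds interactor, policy, critic and trainer from network assets, passing the hero to interactor and trainer.
; A RunInference flag switches Tick between inference and training, and encoder, policy and decoder networks reinitialize when it is off.
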(event `self.ReceiveBeginPlay`
  (bind _returnvalue (not (`self.RunInference`)))
  (`|ExecutionSequence`
    (:`then_0`
      (bind _outactors (`GameplayStatics.GetAllActorsOfClass` "/Game/Rougelike/Blueprints/Characters/Enemy/BP_Scorpion.BP_Scorpion_C"))
      (bind _output_get (set `self.Scorpions` _outactors))
      (`self.AddTickPrerequisiteActor` _output_get self))
    (:`then_1`
      (bind _returnvalue_2 (`GameplayStatics.GetActorOfClass` "/Game/Rougelike/Blueprints/Characters/Hero/BP_HeroCharacter.BP_HeroCharacter_C"))
      (set `self.Hero` _returnvalue_2))
    (:`then_2`
      (bind _returnvalue_3 (`LearningAgentsInteractor.MakeInteractor` (`self.LearningAgentsManager`) "/Game/Rougelike/Blueprints/Characters/Enemy/LearningAgent/BP_LearningAgentsInteractor.BP_LearningAgentsInteractor_C"))
      (bind _output_get_2 (set `self.Interactor` _returnvalue_3))
      (set `/Game/Rougelike/Blueprints/Characters/Enemy/LearningAgent/BP_LearningAgentsInteractor.Hero` (`self.Hero`) _output_get_2))
    (:`then_3`
      (bind _returnvalue_4 (`LearningAgentsPolicy.MakePolicy` (`self.LearningAgentsManager`) (`self.Interactor`) "/Script/LearningAgents.LearningAgentsPolicy" "Policy" "/Game/Rougelike/Blueprints/Characters/Enemy/LearningAgent/DA_Encoder.DA_Encoder" "/Game/Rougelike/Blueprints/Characters/Enemy/LearningAgent/DA_Policy.DA_Policy" "/Game/Rougelike/Blueprints/Characters/Enemy/LearningAgent/DA_Decoder.DA_Decoder" _returnvalue _returnvalue _returnvalue (`self.Policy Settings`)))
      (set `self.Policy` _returnvalue_4))
    (:`then_4`
      (bind _returnvalue_5 (`LearningAgentsCritic.MakeCritic` (`self.LearningAgentsManager`) (`self.Interactor`) (`self.Policy`) "/Script/LearningAgents.LearningAgentsCritic" "Critic" "/Game/Rougelike/Blueprints/Characters/Enemy/LearningAgent/DA_Critic.DA_Critic" true (`self.Critic Settings`)))
      (set `self.Critic` _returnvalue_5))
    (:`then_5`
      (bind _returnvalue_6 (`LearningAgentsTrainer.MakeTrainer` (`self.LearningAgentsManager`) (`self.Interactor`) (`self.Policy`) (`self.Critic`) "/Game/Rougelike/Blueprints/Characters/Enemy/LearningAgent/BP_ScorpionTrainer.BP_ScorpionTrainer_C" "Trainer" (`self.Trainer Settings`)))
      (bind _output_get_3 (set `self.Trainer` _returnvalue_6))
      (set `/Game/Rougelike/Blueprints/Characters/Enemy/LearningAgent/BP_ScorpionTrainer.Hero` (`self.Hero`) _output_get_3))))

(event `self.ReceiveTick`
  (params (DeltaSeconds :type "Float (single-precision)"))
  (if (`self.RunInference`)
    (`LearningAgentsPolicy.RunInference` (`self.Policy`) 1.0)
    (else
      (`LearningAgentsTrainer.RunTraining` (`self.Trainer`) (`self.Trainer Training Settings`) (`self.Trainer Game Settings`) (`self.Trainer Path Settings`) true true))))

(fn `UserConstructionScript`)