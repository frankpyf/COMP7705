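; Learning Agents trainer Blueprint that defines rewards and episode completion for training the BP_Scorpion enemy against the Hero.
; The reward sums a bonus for being near the Hero, a penalty for straying too far and a scaled, unspecified Hero gameplay attribute value.
; Episodes terminate when the Hero dies; a matching check for the scorpion's death exists but is unused.
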(fn `GatherAgentCompletion`
  (params (AgentId :type Integer))
  (returns (OutCompletion :type "ELearningAgentsCompletion Enum"))
  (return (`LearningAgentsCompletions.MakeCompletionOnCondition` (not (`BaseCharacter.IsAlive` (`self.Hero`))) "Termination" "ConditionCompletion" false null)))

(fn `GatherAgentReward`
  (params (AgentId :type Integer))
  (returns (OutReward :type "Float (single-precision)"))
  (bind _returnvalue (`Actor.K2_GetActorLocation` (`self.Hero`)))
  (bind _returnvalue_2 (`Actor.K2_GetActorLocation` (`self.Scorpion`)))
  (set `self.Scorpion` (`self.GetAgent` AgentId "/Game/Rougelike/Blueprints/Characters/Enemy/BP_Scorpion.BP_Scorpion_C"))
  (return (+ (`LearningAgentsRewards.MakeRewardOnLocationDifferenceBelowThreshold` _returnvalue _returnvalue_2 400.0 1.0 "LocationDifferenceBelowThresholdReward" false null) (`LearningAgentsRewards.MakeRewardOnLocationDifferenceAboveThreshold` _returnvalue _returnvalue_2 1000.0 -10.0 "LocationDifferenceAboveThresholdReward" false null) (`LearningAgentsRewards.MakeReward` (`.ReturnValue` (`AbilitySystemComponent.GetGameplayAttributeValue` (`BaseCharacter.GetAbilitySystemComponent` (`self.Hero`)) (struct :`AttributeName` "IncomingDamage" :`Attribute` "/Script/CapstoneProject.CharacterBaseAttributeSet:IncomingDamage" :`AttributeOwner` "/Script/CoreUObject.Class'/Script/CapstoneProject.CharacterBaseAttributeSet'"))) 10.0 "Reward" false null))))