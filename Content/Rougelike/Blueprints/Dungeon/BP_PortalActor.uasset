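; Interactable dungeon portal that streams in a random level and teleports the player between it and a fixed location.
; An Interact while unloaded starts loading a random level from LevelsToLoad and adds a portal plane mesh.
; An Interact while loaded alternates between teleporting above a found BP_Room and returning to fixed coordinates while unloading the last loaded level.
; Both teleports clear the Loaded flag, so each is preceded by a new load.
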(event `InteractInterface.Interact`
  (params (InstigatorPawn :type "Actor Object Reference"))
  (if (`self.bLoaded`)
    (`/Engine/EditorBlueprintResources/StandardMacros.FlipFlop`
      (:`A`
        (bind _returnvalue (`GameplayStatics.GetActorOfClass` "/Game/Rougelike/Blueprints/Dungeon/BP_Room.BP_Room_C"))
        (`self.K2_TeleportTo` :`self` (`GameplayStatics.GetPlayerPawn` 0) :`DestLocation` (+ (`self.K2_GetActorLocation` _returnvalue) (0.0 0.0 200.0)))
        (set `self.bLoaded` false))
      (:`B`
        (`self.K2_TeleportTo` :`self` (`GameplayStatics.GetPlayerPawn` 0) :`DestLocation` (-4620.0 -4770.0 100.0))
        (`GameplayStatics.UnloadStreamLevel` (`self.LoadedLevel`))
        (set `self.bLoaded` false)))
    (else
      (bind _output_get (set `self.LoadedLevel` (`KismetArrayLibrary.Array_Random` (`self.LevelsToLoad`))))
      (`GameplayStatics.LoadStreamLevel` _output_get true)
      (bind _returnvalue_2 (`AddComponent|NODE_AddStaticMeshComponent-0` :`RelativeTransform` (`KismetMathLibrary.MakeTransform` (0.0 0.0 200.0) (struct :`Roll` 90.0) (2.0 3.0 1.0))))
      (`StaticMeshComponent.SetStaticMesh` _returnvalue_2 "/Engine/BasicShapes/Plane.Plane")
      (`PrimitiveComponent.SetMaterial` _returnvalue_2 0 "/Game/Rougelike/Assets/PortalEffects/Portal/M_Portal_2.M_Portal_2")
      (`SceneComponent.K2_AttachToComponent` _returnvalue_2 (`self.MeshComponent`) "None" "KeepRelative" "KeepRelative" "KeepRelative" true)
      (set `self.bLoaded` true))))

(fn `UserConstructionScript`)