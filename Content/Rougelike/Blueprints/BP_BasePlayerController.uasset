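; BP_BasePlayerController is a player controller that stores the possessed hero character and handles the inventory screen toggle.
; The IA_OpenInventory action drives a FlipFlop that alternates between opening and closing the inventory.
; Opening requires a valid, living hero, lazily creates and reuses a WB_Inventory widget, refreshes it and pauses the game.
; Closing removes the widget from the viewport and unpauses.
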(event `self.ReceivePossess`
  (params (PossessedPawn :type "Pawn Object Reference"))
  (bind _asbp_hero_character (cast `/Game/RougeLike/Blueprints/Characters/Hero/BP_HeroCharacter` PossessedPawn))
  (set `self.Hero Character` _asbp_hero_character))

(event `EnhancedInput|/Game/Rougelike/Input/Actions/IA_OpenInventory`
  (params (ActionValue :type Boolean) (ElapsedSeconds :type "Float (double-precision)") (TriggeredSeconds :type "Float (double-precision)") (InputAction :type "InputAction Object Reference" :default "/Game/Rougelike/Input/Actions/IA_OpenInventory.IA_OpenInventory"))
  (bind _hero_character (`self.Hero Character`))
  (bind _inventorywidget (`self.InventoryWidget`))
  (bind _inventorywidget_2 (`self.InventoryWidget`))
  (:`Triggered`
    (`/Engine/EditorBlueprintResources/StandardMacros.FlipFlop`
      (:`A`
        (`/Engine/EditorBlueprintResources/StandardMacros.IsValid` _hero_character
          (:`Is Valid`
            (if (`BaseCharacter.IsAlive` _hero_character)
              (`/Engine/EditorBlueprintResources/StandardMacros.IsValid` (`self.InventoryWidget`)
                (:`Is Valid`
                  _)
                (:`Is Not Valid`
                  (bind _returnvalue (`|CreateWidget` "/Game/Rougelike/UI/Inventory/WB_Inventory.WB_Inventory_C" self))
                  (set `self.InventoryWidget` _returnvalue)))
              (`UserWidget.AddToViewport` _inventorywidget 0)
              (`/Game/Rougelike/UI/Inventory/WB_Inventory.Update Inventory` _inventorywidget)
              (`GameplayStatics.SetGamePaused` true)))))
      (:`B`
        (`/Engine/EditorBlueprintResources/StandardMacros.IsValid` (`self.InventoryWidget`)
          (:`Is Valid`
            (if (`Widget.IsInViewport` _inventorywidget_2)
              (`Widget.RemoveFromParent` _inventorywidget_2)
              (`GameplayStatics.SetGamePaused` false))))))))

(fn `UserConstructionScript`)