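; BP_HUD_Base is a HUD Blueprint that puts the base HUD widget on screen and keeps the hero's health bar up to date.
; On BeginPlay it creates WB_HUD_Base for the owning player, records it in the Widgets array and adds it to the viewport.
; If the owning pawn is a BP_HeroCharacter, it binds to max and current health change events, forwarding new values to the widget's HealthBar.
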(event `self.ReceiveBeginPlay`
  (bind _returnvalue (`|CreateWidget` "/Game/RougeLike/UI/WB_HUD_Base.WB_HUD_Base_C" (`self.GetOwningPlayerController`)))
  (bind _output_get (set `self.Base HUD` _returnvalue))
  (`KismetArrayLibrary.Array_Add` (`self.Widgets`) _output_get)
  (`UserWidget.AddToViewport` _output_get 0)
  (bind _asbp_hero_character (cast `/Game/RougeLike/Blueprints/Characters/Hero/BP_HeroCharacter` (`self.GetOwningPawn`)))
  (add `HeroCharacter.MaxHealthChanged` _asbp_hero_character (delegate `MaxHealthChanged`))
  (add `HeroCharacter.HealthChanged` _asbp_hero_character (delegate `HealthChanged`)))

(event `MaxHealthChanged`
  (params (NewMaxHealth :type "Float (single-precision)"))
  (`/Game/Rougelike/UI/WB_StateBar.UpdateMax` (`/Game/RougeLike/UI/WB_HUD_Base.HealthBar` (`self.Base HUD`)) NewMaxHealth))

(event `HealthChanged`
  (params (NewHealth :type "Float (single-precision)"))
  (`/Game/Rougelike/UI/WB_StateBar.UpdateCurrent` (`/Game/RougeLike/UI/WB_HUD_Base.HealthBar` (`self.Base HUD`)) NewHealth))

(fn `UserConstructionScript`)