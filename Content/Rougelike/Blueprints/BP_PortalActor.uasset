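; An interactable portal actor that moves the player between two fixed locations and streams randomly chosen levels.
; When not loaded, interacting streams in a random level from LevelsToLoad and turns the portal blue.
; When loaded, interacting teleports the player by the IsPreparing state, flips it and clears Loaded, either graying the portal or unloading LoadedLevel.
; The construction script creates the plane's dynamic effect material, initially black.
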(event `self.ReceiveActorBeginOverlap`
  (params (OtherActor :type "Actor Object Reference")))

(event `InteractInterface.Interact`
  (params (InstigatorPawn :type "Actor Object Reference"))
  (if (`self.bLoaded`)
    (if (`self.GetIsPreparing`)
      (`self.K2_TeleportTo` :`self` (`GameplayStatics.GetPlayerPawn` 0) :`DestLocation` (1000.0 1000.0 100.0))
      (`self.FlipIsPreparing`)
      (`MaterialInstanceDynamic.SetVectorParameterValue` (`self.PortalEffectMaterial`) "Color" (struct :`R` 0.044271 :`G` 0.044271 :`B` 0.044271 :`A` 1.0))
      (set `self.bLoaded` false)
      (else
        (`self.K2_TeleportTo` :`self` (`GameplayStatics.GetPlayerPawn` 0) :`DestLocation` (-4620.0 -4770.0 100.0))
        (`self.FlipIsPreparing`)
        (`GameplayStatics.UnloadStreamLevel` (`self.LoadedLevel`))
        (set `self.bLoaded` false)))
    (else
      (bind _output_get (set `self.LoadedLevel` (`KismetArrayLibrary.Array_Random` (`self.LevelsToLoad`))))
      (`GameplayStatics.LoadStreamLevel` _output_get true)
      (`MaterialInstanceDynamic.SetVectorParameterValue` (`self.PortalEffectMaterial`) "Color" (struct :`G` 0.46006 :`B` 0.997396 :`A` 1.0))
      (set `self.bLoaded` true))))

(fn `UserConstructionScript`
  (bind _returnvalue (`PrimitiveComponent.CreateDynamicMaterialInstance` (`self.Plane`) 0 "/Game/Rougelike/Assets/Materials/Portal/MI_PortalEffect.MI_PortalEffect" "None"))
  (bind _output_get (set `self.PortalEffectMaterial` _returnvalue))
  (`MaterialInstanceDynamic.SetVectorParameterValue` _output_get "Color" (struct :`A` 1.0)))