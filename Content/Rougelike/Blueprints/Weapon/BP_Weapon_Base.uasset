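; Base weapon actor that detects melee hits through a capsule collider switched on at attack begin and off shortly after attack end, when its hit list clears.
; Overlaps skip actors of the instigator's own class and those already recorded during the swing.
; A DoOnce, reset shortly after an overlap ends, gates an Event.Attack.WeaponHit gameplay event sent to the instigator with the struck actor as target.
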(event `WeaponBeginAttack`
  (`PrimitiveComponent.SetCollisionEnabled` (`self.Capsule`) "QueryOnly"))

(event `WeaponEndAttack`
  (`KismetSystemLibrary.Delay` 0.1)
  (`PrimitiveComponent.SetCollisionEnabled` (`self.Capsule`) "NoCollision")
  (`KismetArrayLibrary.Array_Clear` (`self.ActorsToIgnore`)))

(event `self.Capsule.OnComponentBeginOverlap`
  (params (OverlappedComponent :type "PrimitiveComponent Object Reference") (OtherActor :type "Actor Object Reference") (OtherComp :type "PrimitiveComponent Object Reference") (OtherBodyIndex :type Integer) (bFromSweep :type Boolean) (SweepResult :type "HitResult Structure (by ref)"))
  (bind _returnvalue (`self.GetInstigator`))
  (bind _actorstoignore (`self.ActorsToIgnore`))
  (if (!= (`GameplayStatics.GetObjectClass` OtherActor) (`GameplayStatics.GetObjectClass` (`self.GetInstigator`)))
    (if (not (`KismetArrayLibrary.Array_IsValidIndex` _actorstoignore (`KismetArrayLibrary.Array_Find` _actorstoignore OtherActor)))
      (`KismetArrayLibrary.Array_Add` (`self.ActorsToIgnore`) OtherActor)
      (`/Engine/EditorBlueprintResources/StandardMacros.DoOnce` false :!label _label
        (:`Completed`
          (`AbilitySystemBlueprintLibrary.SendGameplayEventToActor` _returnvalue (struct :`TagName` "Event.Attack.WeaponHit") (make `GameplayEventData` (struct) _returnvalue OtherActor)))))))

(event `self.Capsule.OnComponentEndOverlap`
  (params (OverlappedComponent :type "PrimitiveComponent Object Reference") (OtherActor :type "Actor Object Reference") (OtherComp :type "PrimitiveComponent Object Reference") (OtherBodyIndex :type Integer))
  (`KismetSystemLibrary.Delay` 0.1)
  (goto _label :!via `Reset`))

(fn `UserConstructionScript`)