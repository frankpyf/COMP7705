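; BP_GameMode_Base is a game mode Blueprint for the roguelike that handles the game-over sequence.
; OnGameOver briefly slows global time as a slow-motion beat, restores normal speed, then pauses the game and switches the first player's input to UI only with the mouse locked.
; It then shows the WB_GameOver widget, creating and caching it in EndingUI only if no valid instance exists.
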(event `self.OnGameOver`
  (`GameplayStatics.SetGlobalTimeDilation` 0.25)
  (`KismetSystemLibrary.Delay` 1.0)
  (`GameplayStatics.SetGlobalTimeDilation` 1.0)
  (`GameplayStatics.SetGamePaused` true)
  (`WidgetBlueprintLibrary.SetInputMode_UIOnlyEx` (`GameplayStatics.GetPlayerController` 0) null "LockAlways")
  (`/Engine/EditorBlueprintResources/StandardMacros.IsValid` (`self.EndingUI`)
    (:`Is Valid`
      _)
    (:`Is Not Valid`
      (bind _returnvalue (`|CreateWidget` "/Game/Rougelike/UI/WB_GameOver.WB_GameOver_C"))
      (set `self.EndingUI` _returnvalue)))
  (`UserWidget.AddToViewport` (`self.EndingUI`) 0))

(fn `UserConstructionScript`)