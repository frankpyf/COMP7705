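; GA_Dash is a Gameplay Ability that dashes a BaseCharacter along its movement input, or backward when there is none.
; After committing, it switches movement to Falling and plays AM_Dash, choosing one of four numbered sections from the dash direction relative to facing.
; A constant root motion force drives the dash for a fraction of the montage length.
; When the force finishes, Walking is restored and the ability ends.
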(event `self.K2_ActivateAbility`
  (bind _returnvalue (`self.GetAvatarActorFromActorInfo`))
  (bind _asbase_character (cast `BaseCharacter` _returnvalue :!pure true))
  (bind _charactermovement (`Character.CharacterMovement` _asbase_character))
  (bind _returnvalue_2 (`CharacterMovementComponent.GetCurrentAcceleration` _charactermovement))
  (bind _returnvalue_3 (`self.K2_CommitAbility`))
  (if _returnvalue_3
    (`CharacterMovementComponent.SetMovementMode` _charactermovement "MOVE_Falling" 0)
    (if (> (`KismetMathLibrary.VSizeXY` _returnvalue_2) 0.0)
      (set `self.Direction` (`KismetMathLibrary.Vector_Normal2D` _returnvalue_2))
      (else
        (set `self.Direction` (`KismetMathLibrary.NegateVector` (`Actor.GetActorForwardVector` _returnvalue)))))
    (`AbilityTask_PlayMontageAndWait.CreatePlayMontageAndWaitProxy` "None" "/Game/Rougelike/Assets/Characters/Mannequins/Animations/Manny/Dash/AM_Dash.AM_Dash" 1.5 (`self.GetMontageSection` (`Actor.K2_GetActorRotation` _asbase_character))
      (:`then`
        (`AbilityTask_ApplyRootMotionConstantForce.ApplyRootMotionConstantForce` "None" (`self.Direction`) 900.0 (/ (`AnimSequenceBase.SequenceLength` (`self.GetCurrentMontage`)) 8.0) false null "MaintainLastRootMotionVelocity" (0.0 0.0 0.0) 1000.0
          (:`OnFinish`
            (`CharacterMovementComponent.SetMovementMode` _charactermovement "MOVE_Walking" 0)
            (`self.K2_EndAbility`)))))))

(fn `GetMontageSection`
  (params (BaseRotation :type "Rotator Structure"))
  (returns (SectionName :type Name))
  (return (`KismetStringLibrary.Conv_StringToName` (`KismetStringLibrary.Conv_IntToString` (mod (`KismetMathLibrary.Round` (/ (`KismetMathLibrary.ClampAxis` (`KismetAnimationLibrary.CalculateDirection` (`self.Direction`) BaseRotation)) 90.0)) 4)))))